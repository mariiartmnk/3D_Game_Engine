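; BP_BusObject is a bus actor that travels along a referenced spline actor's path, starting at BeginPlay.
; A timeline, with play rate set from TimeToComplete, drives an alpha that is lerped over the spline's length.
; Each update samples world-space location and rotation at that distance and applies both to the actor.
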(event Custom|MoveObject
  (bind _splinetofollow (Variables|Default|GetSplineToFollow))
  (bind _spline (Variables|/Game/BP_BusPath.BP_BusPath_C|GetSpline _splinetofollow))
  ;[0.15 0.15 0.15 0.5] Bus Spline Moving Logic
  (Components|Timeline|SetPlayRate (Variables|Default|GetT_Move) (/ 1.0 (Variables|Default|GetTimeToComplete)))
  (bind _movetrack (Timeline|T_Move Play)
    (:Update
      (Transformation|SetActorLocationAndRotation (Spline|GetLocationatDistanceAlongSpline _spline (Math|Float|Lerp 0.0 (Spline|GetSplineLength _spline) _movetrack) "World") (Spline|GetRotationatDistanceAlongSpline _spline (Math|Float|Lerp 0.0 (Spline|GetSplineLength _spline) _movetrack) "World")))))

(event EventBeginPlay
  ;[0.15 0.15 0.15 0.5] Bus Spline Moving Logic
  (CallFunction|MoveObject))

(fn ConstructionScript)